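; Cube capture actor for parallax-corrected cubemaps that renders its surroundings into a target texture.
; The construction script applies the texture and every-frame setting to the capture component.
; When per-frame capture is off, a custom event nudges the component along Z to force a one-shot capture.
; Helper functions derive the projection box from the actor transform, as an AABB or as OBB world-to-local inverse matrix vectors.
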(event Custom|EventCaptureOneShot
  (bind _cubecapture (Variables|Default|GetCubeCapture))
  ;[1 1 1] 毎フレームキャプチャが有効でない場合、この命令で1ショットだけキャプチャを行う
  (if (not (Variables|Capture|GetCaptureEveryFrame))
    ;;[1 1 1] 位置を移動させるとキャプチャされる
    (Transformation|SetRelativeLocation _cubecapture "0, 0,-0.100000" false)
    (Transformation|SetRelativeLocation _cubecapture "0, 0,0.100000" false)))

(event EventBeginPlay)

(event EventActorBeginOverlap
  (params (OtherActor :type Actor%20Object%20Reference)))

(event EventTick
  (params (DeltaSeconds :type Float%20%28single-precision%29)))

(fn ConstructionScript
  (bind _cubecapture (Variables|Default|GetCubeCapture))
  (Variables|/Script/Engine.SceneCaptureComponentCube|SetTextureTarget _cubecapture (Variables|Capture|GetTargetTexture))
  (Variables|/Script/Engine.SceneCaptureComponent|SetbCaptureEveryFrame _cubecapture (Variables|Capture|GetCaptureEveryFrame)))

(fn GetCubeAABB
  (bind _returnvalue (Transformation|GetActorScale3D))
  (bind _returnvalue_2 (Transformation|GetActorLocation))
  (return (- _returnvalue_2 _returnvalue) (+ _returnvalue_2 _returnvalue)))

(fn GetOBBWorldtoLocal
  (bind _returnvalue (Transformation|GetActorLocation))
  (bind _returnvalue_2 (Transformation|GetActorRotation))
  (bind _returnvalue_3 (Transformation|GetActorScale3D))
  (bind (_x _y _z) (Math|Rotator|BreakRotIntoAxes _returnvalue_2))
  (bind _returnvalue_4 (/ "1.000000,1.000000,1.000000" _returnvalue_3))
  (bind _returnvalue_5 (* _returnvalue -1.0))
  (bind (_x_2 _y_2 _z_2) (Math|Vector|BreakVector _returnvalue_4))
  (bind _returnvalue_6 (* _z _z_2))
  (bind _returnvalue_7 (* _x _x_2))
  (bind _returnvalue_8 (* _y _y_2))
  (return _returnvalue_7 _returnvalue_8 _returnvalue_6 (Math|Vector|MakeVector (Math|Vector|DotProduct _returnvalue_5 _returnvalue_7) (Math|Vector|DotProduct _returnvalue_5 _returnvalue_8) (Math|Vector|DotProduct _returnvalue_5 _returnvalue_6))))