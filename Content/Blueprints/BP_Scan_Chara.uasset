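; BP_Scan_Chara is a movable character whose mesh material shows a scan effect relative to an assigned plane actor.
; The construction script creates a dynamic instance of M_Scan_Destination, and input axes move the character along world X and Y.
; SetPlaneEvent stores the plane actor and toggles the material's Line parameter by its validity.
; Each tick feeds that plane's position and up vector to the material as PlanePos and PlaneNormal.
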(event Custom|SetPlaneEvent
  (params (ScanPlane :type Actor%20Object%20Reference))
  (bind _materialinst (Variables|Default|GetMaterialInst))
  (Variables|Default|SetScanPlaneActor ScanPlane)
  (Utilities|IsValid ScanPlane
    (:Is%20Valid
      (Rendering|Material|SetScalarParameterValue _materialinst "Line" 1.0 :!class /Script/Engine.MaterialInstanceDynamic))
    (:Is%20Not%20Valid
      (Rendering|Material|SetScalarParameterValue _materialinst "Line" 0.0 :!class /Script/Engine.MaterialInstanceDynamic))))

(event EventTick
  (params (DeltaSeconds :type Float%20%28single-precision%29))
  (bind _materialinst (Variables|Default|GetMaterialInst))
  (bind _scanplaneactor (Variables|Default|GetScanPlaneActor))
  (bind _returnvalue (Transformation|GetActorTransform _scanplaneactor))
  (bind (_location _rotation) (Math|Transform|BreakTransform _returnvalue))
  (Utilities|IsValid _scanplaneactor
    (:Is%20Valid
      (Rendering|Material|SetVectorParameterValue _materialinst "PlanePos" (Math|Conversions|ToLinearColor(Vector) _location) :!class /Script/Engine.MaterialInstanceDynamic)
      (Rendering|Material|SetVectorParameterValue _materialinst "PlaneNormal" (Math|Conversions|ToLinearColor(Vector) (.Z (Math|Rotator|GetAxes _rotation))) :!class /Script/Engine.MaterialInstanceDynamic))))

(event Input|AxisEvents|InputAxisKeyRight
  (params (AxisValue :type Float%20%28single-precision%29))
  (Pawn|Input|AddMovementInput "0,1.000000, 0" AxisValue false))

(event Input|AxisEvents|InputAxisKeyUp
  (params (AxisValue :type Float%20%28single-precision%29))
  (Pawn|Input|AddMovementInput "1.000000, 0, 0" AxisValue false))

(fn ConstructionScript
  (bind _returnvalue (Rendering|Material|CreateDynamicMaterialInstance 0 "/Game/Materials/Samples/M_Scan_Destination.M_Scan_Destination" :!class /Script/Engine.PrimitiveComponent))
  (Variables|Default|SetMaterialInst _returnvalue))