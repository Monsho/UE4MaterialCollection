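; BP_Scan_Plane is an actor that displays a scan effect shaped by a length, an angle and the actor's facing.
; The construction script creates a dynamic instance of MI_Scan_Plane and passes it ScanLength, ScanAngle and the forward vector, converted to a color.
; Tick pushes the same three parameters every frame, so the material follows runtime changes in rotation and scan values.
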(event EventTick
  (params (DeltaSeconds :type Float%20%28single-precision%29))
  (bind _material (Variables|Default|GetMaterial))
  (Rendering|Material|SetScalarParameterValue _material "Length" (Variables|Default|GetScanLength) :!class /Script/Engine.MaterialInstanceDynamic)
  (Rendering|Material|SetVectorParameterValue _material "Front" (Math|Conversions|ToLinearColor(Vector) (.X (Math|Rotator|GetAxes (Transformation|GetActorRotation)))) :!class /Script/Engine.MaterialInstanceDynamic)
  (Rendering|Material|SetScalarParameterValue _material "Angle" (Variables|Default|GetScanAngle) :!class /Script/Engine.MaterialInstanceDynamic))

(fn ConstructionScript
  (bind _returnvalue (Rendering|Material|CreateDynamicMaterialInstance 0 "/Game/Materials/Samples/Instances/MI_Scan_Plane.MI_Scan_Plane" :!class /Script/Engine.PrimitiveComponent))
  (Variables|Default|SetMaterial _returnvalue)
  (Rendering|Material|SetScalarParameterValue _returnvalue "Length" (Variables|Default|GetScanLength) :!class /Script/Engine.MaterialInstanceDynamic)
  (Rendering|Material|SetVectorParameterValue _returnvalue "Front" (Math|Conversions|ToLinearColor(Vector) (.X (Math|Rotator|GetAxes (Transformation|GetActorRotation)))) :!class /Script/Engine.MaterialInstanceDynamic)
  (Rendering|Material|SetScalarParameterValue _returnvalue "Angle" (Variables|Default|GetScanAngle) :!class /Script/Engine.MaterialInstanceDynamic))